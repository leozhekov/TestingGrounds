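; NPC AI Blueprint that drives guard behavior through a behavior tree and perception.
; On BeginPlay it sets up the Patrol_Data blackboard and runs the GuardBehaviour tree.
; Perception updates write any sensed actor lacking the "Enemy" tag to the Enemy blackboard key.
; The key is cleared when such an actor is no longer sensed, without checking whether it is the stored one.
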(event `self.ReceiveBeginPlay`
  (bind _blackboardcomponent (`self.UseBlackboard` "/Game/Dynamic/NPC/AI/Patrol_Data.Patrol_Data"))
  (`self.RunBehaviorTree` "/Game/Dynamic/NPC/AI/GuardBehaviour.GuardBehaviour")
  (set `self.BlackboardComp` _blackboardcomponent))

(event `self.AIPerception.OnTargetPerceptionUpdated`
  (params (Actor :type "Actor Object Reference") (Stimulus :type "AIStimulus Structure"))
  (if (`self.ActorHasTag` Actor "Enemy")
    _
    (elif (`.bSuccessfullySensed` (break `AIStimulus` Stimulus))
      (`BlackboardComponent.SetValueAsObject` (`self.BlackboardComp`) (`self.Enemy`) Actor)
      (else
        (`BlackboardComponent.ClearValue` (`self.BlackboardComp`) (`self.Enemy`))))))

(fn `UserConstructionScript`)