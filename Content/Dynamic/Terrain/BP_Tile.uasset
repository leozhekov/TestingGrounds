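; BP_Tile is a terrain tile for an infinite terrain mode that scatters canisters, containers, rocks and sandbags via PlaceActors on BeginPlay.
; Its barrier starts locked, opens in green when the player enters LockingVolume, and turns solid red when they leave.
; Leaving that volume also asks InfiniteTerrainGameMode to spawn another tile, with GetAttatchLocation exposing the Arrow's transform.
; The tile destroys itself when the player enters DestroyVolume.
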(event `self.ReceiveBeginPlay`
  (`self.Lock`)
  (`self.PlaceActors` "/Game/Dynamic/Terrain/Props/BP_Canister.BP_Canister_C" 1 5 50.0)
  (`self.PlaceActors` "/Game/Dynamic/Terrain/Props/BP_Container.BP_Container_C" 1 2 450.0)
  (`self.PlaceActors` "/Game/Dynamic/Terrain/Props/BP_Rock_2.BP_Rock_2_C" 1 3 250.0 1.0 5.0)
  (`self.PlaceActors` "/Game/Dynamic/Terrain/Props/BP_Rock_3.BP_Rock_3_C" 0 4 250.0 1.0 5.0)
  (`self.PlaceActors` "/Game/Dynamic/Terrain/Props/BP_Sandbags.BP_Sandbags_C" 1 2 250.0))

(event `self.Locking volume.OnComponentBeginOverlap`
  (params (OverlappedComponent :type "PrimitiveComponent Object Reference") (OtherActor :type "Actor Object Reference") (OtherComp :type "PrimitiveComponent Object Reference") (OtherBodyIndex :type Integer) (bFromSweep :type Boolean) (SweepResult :type "HitResult Structure (by ref)"))
  (`self.Is player` OtherActor)
  (`self.Unlock`))

(event `self.Locking volume.OnComponentEndOverlap`
  (params (OverlappedComponent :type "PrimitiveComponent Object Reference") (OtherActor :type "Actor Object Reference") (OtherComp :type "PrimitiveComponent Object Reference") (OtherBodyIndex :type Integer))
  (`self.Is player` OtherActor)
  (`self.Lock`)
  (bind _asinfinite_terrain_game_mode (cast `/Game/Dynamic/InfiniteTerrainGameMode` (`GameplayStatics.GetGameMode`)))
  (`/Game/Dynamic/InfiniteTerrainGameMode.Spawn Tile` _asinfinite_terrain_game_mode))

(event `self.Destroy Volume.OnComponentBeginOverlap`
  (params (OverlappedComponent :type "PrimitiveComponent Object Reference") (OtherActor :type "Actor Object Reference") (OtherComp :type "PrimitiveComponent Object Reference") (OtherBodyIndex :type Integer) (bFromSweep :type Boolean) (SweepResult :type "HitResult Structure (by ref)"))
  (`self.Is player` OtherActor)
  (`self.K2_DestroyActor`))

(fn `GetAttatchLocation`
  (returns (`Attach Transform` :type "Transform Structure"))
  (return (`SceneComponent.K2_GetComponentToWorld` (`self.Arrow`))))

(fn `Lock`
  (`PrimitiveComponent.SetCollisionEnabled` (`self.Barrier`) "QueryAndPhysics")
  (`PrimitiveComponent.SetMaterial` (`self.Barrier`) 0 "/Game/Dynamic/Terrain/MI_Barrier_Red.MI_Barrier_Red"))

(fn `Unlock`
  (`PrimitiveComponent.SetCollisionEnabled` (`self.Barrier`) "NoCollision")
  (`PrimitiveComponent.SetMaterial` (`self.Barrier`) 0 "/Game/Dynamic/Terrain/MI_Barrier_Green.MI_Barrier_Green"))

(fn `UserConstructionScript`)