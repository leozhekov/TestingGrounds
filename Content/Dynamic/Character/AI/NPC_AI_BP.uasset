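; NPC AI controller that drives a guard character using the GuardBehaviour behavior tree and Patrol_Data blackboard.
; AI perception updates write any sensed actor lacking the "Enemy" tag into the blackboard's Enemy key, and clear that key when such an actor is lost.
; Each tick, the controlled BP_Character's aiming and shooting flags follow whether the controller has a valid focus actor.
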(event `self.ReceiveBeginPlay`
  (bind _blackboardcomponent (`self.UseBlackboard` "/Game/Dynamic/Character/AI/Patrol_Data.Patrol_Data"))
  (`self.RunBehaviorTree` "/Game/Dynamic/Character/AI/GuardBehaviour.GuardBehaviour")
  (set `self.BlackboardComp` _blackboardcomponent))

(event `self.AIPerception.OnTargetPerceptionUpdated`
  (params (Actor :type "Actor Object Reference") (Stimulus :type "AIStimulus Structure"))
  (`self.Update Blackboard Enemy key` Actor Stimulus))

(event `self.ReceiveTick`
  (params (DeltaSeconds :type "Float (single-precision)"))
  (bind _returnvalue (`KismetSystemLibrary.IsValid` (`self.GetFocusActor`)))
  (bind _asbp_character (cast `/Game/Dynamic/Character/Behavior/BP_Character` (`self.K2_GetPawn`)))
  (set `/Game/Dynamic/Character/Behavior/BP_Character.IsAiming` _returnvalue _asbp_character)
  (set `/Game/Dynamic/Character/Behavior/BP_Character.IsShooting` _returnvalue _asbp_character))

(fn `Update Blackboard Enemy key`
  (params (`Detected Actor` :type "Actor Object Reference") (AIStimulus :type "AIStimulus Structure (by ref)"))
  (locals (Actor :type "Actor Object Reference"))
  (bind _output_get (set `local.Actor` `Detected Actor`))
  (if (`self.ActorHasTag` _output_get "Enemy")
    _
    (elif (`.bSuccessfullySensed` (break `AIStimulus` AIStimulus))
      (`BlackboardComponent.SetValueAsObject` (`self.BlackboardComp`) (`self.Enemy`) (`local.Actor`))
      (else
        (`BlackboardComponent.ClearValue` (`self.BlackboardComp`) (`self.Enemy`))))))

(fn `UserConstructionScript`)